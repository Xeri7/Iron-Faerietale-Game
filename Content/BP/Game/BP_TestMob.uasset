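; BP_TestMob is a test mob character whose name and base health come from JSON character templates held by the game mode.
; On authority, BeginPlay polls the game mode every five seconds until data exists, matches TemplateId, then seeds HWCombatAttributeSet health through the ability system.
; Remote instances relink the nameplate widget at BeginPlay.
; Taking damage prints a debug message and updates the nameplate's health percentage and bar.
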(event EventBeginPlay
  (bind _characterdata (Variables|Default|GetCharacterData))
  (Networking|SwitchHasAuthority
    (:Authority
      (|SetupCharacterFromMode)
      (bind _outvalue (|GetJsonField _characterdata "charTemplateName"))
      (Variables|Default|SetCharacterName _outvalue)
      (bind _returnvalue (GameplayAttributes|GetAttributeSet (Variables|Default|GetAbilitySystem) "/Script/OWSHubWorldMMO.HWCombatAttributeSet"))
      (bind _ashwcombat_attribute_set (Utilities|Casting|CastToHWCombatAttributeSet _returnvalue))
      (bind _outvalue_2 (|GetJsonField _characterdata "charForm"))
      (bind _outvalue_3 (|GetJsonField _outvalue_2 "baseHealth"))
      (Class|HWCombatAttributeSet|HWSetMaxHealth _ashwcombat_attribute_set _outvalue_3)
      (Class|HWCombatAttributeSet|HWSetHealth _ashwcombat_attribute_set _outvalue_3)
      (Pawn|Components|CharacterMovement|SetMovementMode (Variables|Character|GetCharacterMovement) "MOVE_Walking" 0))
    (:Remote
      (Class|HWMobNameplateWidgetComponent|RefreshLinktoParent (Variables|Default|GetMobNameplateWidgetComponent)))))

(event EventTick
  (params (DeltaSeconds :type Float%20%28single-precision%29))
  (Networking|SwitchHasAuthority))

(event EventOnTakeDamage
  (params (WhoAttackedMe :type HWGAS%20Character%20Object%20Reference) (DamageAmount :type Float%20%28single-precision%29) (IsCritical :type Boolean))
  (bind _mobnameplatewidgetcomponent (Variables|Default|GetMobNameplateWidgetComponent))
  (bind _returnvalue (UserInterface|GetUserWidgetObject _mobnameplatewidgetcomponent))
  (bind _asmob_nameplate_widget (Utilities|Casting|CastToMobNameplateWidget _returnvalue))
  (Development|PrintString "OUCH")
  (bind _returnvalue_2 (GameplayAttributes|GetAttributeSet (Variables|Default|GetAbilitySystem) "/Script/OWSHubWorldMMO.HWCombatAttributeSet"))
  (bind _ashwcombat_attribute_set (Utilities|Casting|CastToHWCombatAttributeSet _returnvalue_2))
  (Class|HWMobNameplateWidgetComponent|RefreshLinktoParent _mobnameplatewidgetcomponent)
  (Variables|/Script/UMG.TextBlock|SetText (Variables|/Game/BP/HUD/MobNameplate/MobNameplateWidget.MobNameplateWidget_C|GetHP _asmob_nameplate_widget) (Utilities|Text|ToText(String) (Utilities|String|Append (Utilities|String|ToString(Integer) (Math|Float|Round (* (/ (Class|HWCombatAttributeSet|HWGetHealth _ashwcombat_attribute_set) (Class|HWCombatAttributeSet|HWGetMaxHealth _ashwcombat_attribute_set)) 1e+02))) "%")))
  (Progress|SetPercent (Variables|/Game/BP/HUD/MobNameplate/MobNameplateWidget.MobNameplateWidget_C|GetHealthBar _asmob_nameplate_widget) (/ (Class|HWCombatAttributeSet|HWGetHealth _ashwcombat_attribute_set) (Class|HWCombatAttributeSet|HWGetMaxHealth _ashwcombat_attribute_set))))

(fn ConstructionScript)