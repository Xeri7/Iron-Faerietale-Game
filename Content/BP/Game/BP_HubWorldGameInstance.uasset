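; BP_HubWorldGameInstance is a game instance Blueprint that shows and hides a full-screen loading dialog.
; RPGBeginLoadingScreen skips dedicated servers, waits one tick, then creates UI_FullScreenLoadingDialog for player controller 0, stores it and adds it to the viewport.
; RPGEndLoadingScreen is empty, so the dialog stays up until the separate HideLoadingDialog event removes the stored widget.
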(event EventRPGBeginLoadingScreen
  (bind _returnvalue (Game|GetPlayerController 0))
  (if (not (Networking|IsDedicatedServer))
    (Utilities|FlowControl|DelayUntilNextTick)
    (Utilities|IsValid _returnvalue
      (:Is%20Valid
        (bind _returnvalue_2 (UserInterface|CreateWidget "/Game/BP/Login/UI_FullScreenLoadingDialog.UI_FullScreenLoadingDialog_C" _returnvalue))
        (Utilities|IsValid _returnvalue_2
          (:Is%20Valid
            (bind _output_get (Variables|Default|SetLoadingScreenWidget _returnvalue_2))
            (UserInterface|Viewport|AddtoViewport _output_get 0)))))))

(event EventRPGEndLoadingScreen)

(event EventHideLoadingDialog
  (bind _loadingscreenwidget (Variables|Default|GetLoadingScreenWidget))
  (Utilities|IsValid _loadingscreenwidget
    (:Is%20Valid
      (Widget|RemovefromParent _loadingscreenwidget))))